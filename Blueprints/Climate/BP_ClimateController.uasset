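; Climate controller actor for seasonal change through MP_Global material parameters, though as wired it only plays woodland ambience on BeginPlay.
; An unconnected delay loop cycles autumn, leaf-fall, snow and spring targets, and a separate unconnected node sets SnowBias.
; The ParameterUpdate graph steps a named collection parameter toward a target by TransitionSpeed until within a small tolerance, but nothing here calls it and Tick is empty.
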(event EventBeginPlay
  (Audio|PlaySound2D "/Game/Audio/Ambience/Ambience_Woodland.Ambience_Woodland" 1.0 1.0 0.0 0 0))

(event Collision|EventActorBeginOverlap
  (params (OtherActor :type Actor%20Object%20Reference)))

(event EventTick
  (params (DeltaSeconds :type Float%20%28single-precision%29)))

(fn ConstructionScript)