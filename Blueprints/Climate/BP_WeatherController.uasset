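; BP_WeatherController is a weather controller that drives sky gloom, cloud opacity and rain.
; Each Tick steps the MP_Global Gloom and RainLevel parameters and sky cloud opacity toward targets by ChangeRate, unscaled by delta time, then updates the skybox.
; ToggleRain switches rain particles and thunder audio and sets the rain target.
; RainLevel's direction check uses Abs, so it only steps upward; a timed weather sequence is left unconnected.
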(event Custom|ToggleRain
  (params (Enable :type Boolean))
  ;[1 1 1] Toggle Rain
  (if Enable
    (Components|Activation|SetActive (Variables|Default|GetP_Rain) true false)
    (Audio|Components|Audio|Play (Variables|Default|Get101509__earthsounds__thunder-and-rain) 0.0)
    (Variables|Default|SetTargetRainLevel 0.9)
    (else
      (Components|Activation|SetActive (Variables|Default|GetP_Rain) false false)
      (Audio|Components|Audio|Stop (Variables|Default|Get101509__earthsounds__thunder-and-rain))
      (Variables|Default|SetTargetRainLevel 0.0))))

(event EventBeginPlay)

(event Collision|EventActorBeginOverlap
  (params (OtherActor :type Actor%20Object%20Reference)))

(event EventTick
  (params (DeltaSeconds :type Float%20%28single-precision%29))
  ;[1 1 1] Update Skybox
  (|UpdateSkyColor
    (:OutputPin
      (|UpdateSkyN
        (:OutputPin
          (|RainLevel_N
            (:OutputPin
              (Default|UpdateSkybox (Variables|Default|GetSky)))))))))

(fn ConstructionScript)